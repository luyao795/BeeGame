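; BP_Swarm is a controllable pawn with yaw-relative planar movement, mouse-look style controller input and a Sphere component that constantly changes shape.
; Each Tick plays a timeline whose alpha blends two interpolations from the current scale toward random per-axis targets, one larger and slower, one smaller and faster, giving an irregular wobble.
; The initial scale is saved at BeginPlay but never read, and the EnableInput call is unconnected.
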(event `self.ReceiveBeginPlay`
  (set `self.InitScale` (`SceneComponent.K2_GetComponentScale` (`self.Sphere`))))

(event `self.ReceiveTick`
  (params (DeltaSeconds :type "Float (single-precision)"))
  (bind _returnvalue (`SceneComponent.K2_GetComponentScale` (`self.Sphere`)))
  ;[1 1 1] Comment
  (bind (_direction _alpha) (`Timeline|Timeline_0`)
    (:`Update`
      (`SceneComponent.SetRelativeScale3D` (`self.Sphere`) (`KismetMathLibrary.VLerp` (`KismetMathLibrary.VInterpTo` _returnvalue (`KismetMathLibrary.MakeVector` (`KismetMathLibrary.RandomFloatInRange` 1.0 3.0) (`KismetMathLibrary.RandomFloatInRange` 1.0 3.0) (`KismetMathLibrary.RandomFloatInRange` 1.0 3.0)) DeltaSeconds 2.0) (`KismetMathLibrary.VInterpTo` _returnvalue (`KismetMathLibrary.MakeVector` (`KismetMathLibrary.RandomFloatInRange` 0.5 1.0) (`KismetMathLibrary.RandomFloatInRange` 0.5 1.0) (`KismetMathLibrary.RandomFloatInRange` 0.5 1.0)) DeltaSeconds 5.0) _alpha)))))

(event `InputAxis|MoveForward` :overrideparent false
  (params (AxisValue :type "Float (single-precision)"))
  ;[1 1 1] Comment
  (`self.AddMovementInput` (`KismetMathLibrary.GetForwardVector` (`KismetMathLibrary.MakeRotator` 0.0 0.0 (.yaw (`self.GetControlRotation`)))) AxisValue))

(event `InputAxis|Turn` :overrideparent false
  (params (AxisValue :type "Float (single-precision)"))
  ;[1 1 1] Comment
  (`self.AddControllerYawInput` AxisValue))

(event `InputAxis|LookUp` :overrideparent false
  (params (AxisValue :type "Float (single-precision)"))
  ;[1 1 1] Comment
  (`self.AddControllerPitchInput` AxisValue))

(event `InputAxis|MoveRight` :overrideparent false
  (params (AxisValue :type "Float (single-precision)"))
  ;[1 1 1] Comment
  (`self.AddMovementInput` (`KismetMathLibrary.GetRightVector` (`KismetMathLibrary.MakeRotator` 0.0 0.0 (.yaw (`self.GetControlRotation`)))) AxisValue))

(fn `UserConstructionScript`)