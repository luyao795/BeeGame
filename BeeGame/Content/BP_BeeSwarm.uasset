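; Bee swarm actor that makes its static mesh pulse and jitter in scale, apparently to mimic a restless swarm.
; Tick plays a timeline whose alpha blends two interpolations from the current world scale, one toward random larger per-axis targets and a faster one toward smaller ones.
; The result sets the mesh's relative scale.
; BeginPlay stores an initial scale, unused afterwards, and enables input for player 0.
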(event `self.ReceiveBeginPlay`
  ;[1 1 1] Comment
  (set `self.InitScale` (`SceneComponent.K2_GetComponentScale` (`self.StaticMeshComponent`)))
  (`self.EnableInput` (`GameplayStatics.GetPlayerController` 0)))

(event `self.ReceiveTick`
  (params (DeltaSeconds :type "Float (single-precision)"))
  (bind _returnvalue (`SceneComponent.K2_GetComponentScale` (`self.StaticMeshComponent`)))
  ;[1 1 1] Comment
  (bind (_direction _alpha) (`Timeline|B/t 0 and 1`)
    (:`Update`
      (`SceneComponent.SetRelativeScale3D` (`self.StaticMeshComponent`) (`KismetMathLibrary.VLerp` (`KismetMathLibrary.VInterpTo` _returnvalue (`KismetMathLibrary.MakeVector` (`KismetMathLibrary.RandomFloatInRange` 1.0 3.0) (`KismetMathLibrary.RandomFloatInRange` 1.0 3.0) (`KismetMathLibrary.RandomFloatInRange` 1.0 3.0)) DeltaSeconds 2.0) (`KismetMathLibrary.VInterpTo` _returnvalue (`KismetMathLibrary.MakeVector` (`KismetMathLibrary.RandomFloatInRange` 0.5 1.0) (`KismetMathLibrary.RandomFloatInRange` 0.5 1.0) (`KismetMathLibrary.RandomFloatInRange` 0.5 1.0)) DeltaSeconds 5.0) _alpha)))))

(fn `UserConstructionScript`)